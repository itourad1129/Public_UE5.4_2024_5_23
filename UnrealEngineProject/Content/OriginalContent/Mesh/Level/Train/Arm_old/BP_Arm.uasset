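; BP_Arm is a train-level mechanical arm actor that switches animation states in response to overlaps.
; ExeArmAnimation writes the requested state to ABP_TrainArm and records it, starting with an initial state on anim init.
; Characters entering the trigger boxes change the state unless ArmHit is set by the body capsule, whose end overlap triggers another state.
; A stop box follows the arm-tip socket every Tick and switches state upon touching static mesh components.
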(event `self.ReceiveBeginPlay`)

(event `self.ArmMesh.OnAnimInitialized`
  (bind _outputanimationtype (`self.ExeArmAnimation` "NewEnumerator4"))
  (set `self.ExecutedAnimationType` _outputanimationtype))

(event `self.ReceiveTick`
  (params (DeltaSeconds :type "Float (single-precision)"))
  (bind _armstopbox (`self.ArmStopBox`))
  (bind (_returnvalue_location _returnvalue_rotation _returnvalue_scale) (`KismetMathLibrary.BreakTransform` (`SceneComponent.K2_GetComponentToWorld` _armstopbox)))
  (`SceneComponent.K2_SetWorldTransform` _armstopbox (`KismetMathLibrary.MakeTransform` (`SceneComponent.GetSocketLocation` (`self.ArmMesh`) "Bone_002_end _socket") _returnvalue_rotation _returnvalue_scale) false false))

(event `self.ArmAnimBox.OnComponentBeginOverlap`
  (params (OverlappedComponent :type "PrimitiveComponent Object Reference") (OtherActor :type "Actor Object Reference") (OtherComp :type "PrimitiveComponent Object Reference") (OtherBodyIndex :type Integer) (bFromSweep :type Boolean) (SweepResult :type "HitResult Structure (by ref)"))
  (cast `Character` OtherActor)
  (if (`self.ArmHit`)
    _
    (elif (!= 1 (`self.ExecutedAnimationType`))
      (bind _outputanimationtype (`self.ExeArmAnimation` "NewEnumerator5"))
      (set `self.ExecutedAnimationType` _outputanimationtype))))

(event `self.ArmBodyCapsule.OnComponentBeginOverlap`
  (params (OverlappedComponent :type "PrimitiveComponent Object Reference") (OtherActor :type "Actor Object Reference") (OtherComp :type "PrimitiveComponent Object Reference") (OtherBodyIndex :type Integer) (bFromSweep :type Boolean) (SweepResult :type "HitResult Structure (by ref)"))
  (set `self.ArmHit` true))

(event `self.ArmBodyCapsule.OnComponentEndOverlap`
  (params (OverlappedComponent :type "PrimitiveComponent Object Reference") (OtherActor :type "Actor Object Reference") (OtherComp :type "PrimitiveComponent Object Reference") (OtherBodyIndex :type Integer))
  (if (`self.ArmHit`)
    (set `self.ArmHit` false)
    (bind _outputanimationtype (`self.ExeArmAnimation` "NewEnumerator6"))
    (set `self.ExecutedAnimationType` _outputanimationtype)))

(event `self.ArmStopBox.OnComponentBeginOverlap`
  (params (OverlappedComponent :type "PrimitiveComponent Object Reference") (OtherActor :type "Actor Object Reference") (OtherComp :type "PrimitiveComponent Object Reference") (OtherBodyIndex :type Integer) (bFromSweep :type Boolean) (SweepResult :type "HitResult Structure (by ref)"))
  (cast `StaticMeshComponent` OtherComp)
  (bind _outputanimationtype (`self.ExeArmAnimation` "NewEnumerator7"))
  (set `self.ExecutedAnimationType` _outputanimationtype))

(event `self.ArmAnimBoxRoot.OnComponentBeginOverlap`
  (params (OverlappedComponent :type "PrimitiveComponent Object Reference") (OtherActor :type "Actor Object Reference") (OtherComp :type "PrimitiveComponent Object Reference") (OtherBodyIndex :type Integer) (bFromSweep :type Boolean) (SweepResult :type "HitResult Structure (by ref)"))
  (cast `Character` OtherActor)
  (if (not (`self.ArmHit`))
    (bind _outputanimationtype (`self.ExeArmAnimation` "NewEnumerator5"))
    (set `self.ExecutedAnimationType` _outputanimationtype)))

(fn `ExeArmAnimation`
  (params (InputAnimationType :type "/Engine/ArtTools/RenderToTexture/Enums/EIntTypes Enum" :default "NewEnumerator4"))
  (returns (OutPutAnimationType :type "/Engine/ArtTools/RenderToTexture/Enums/EIntTypes Enum"))
  (bind _asabp_train_arm (cast `/Game/OriginalContent/Mesh/Level/Train/Arm_old/ABP_TrainArm` (`SkeletalMeshComponent.GetAnimInstance` (`self.ArmMesh`))))
  (bind _output_get (set `/Game/OriginalContent/Mesh/Level/Train/Arm_old/ABP_TrainArm.ArmAnimSwitch` (`local.InputAnimationType`) _asabp_train_arm))
  (return _output_get))

(fn `UserConstructionScript`)